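; BP_TestEnemy is a stand-in enemy that dies automatically three seconds after it begins play, apparently for testing a wave manager.
; AssignWaveManager stores the manager reference that the death event uses.
; After the delay, the 上报死亡 (report death) event calls ReportEnemyDeath on that manager with itself, then destroys the actor.
; IsWaveRelevant always returns false.
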(event Custom|上报死亡
  (Class|WaveManagerComponent|ReportEnemyDeath (Variables|Default|GetMyManager) self)
  (Actor|DestroyActor))

(event EventBeginPlay
  (Utilities|FlowControl|Delay 3.0)
  (CallFunction|上报死亡))

(event EventAssignWaveManager
  (params (Manager :type Wave%20Manager%20Component%20Object%20Reference))
  (Variables|Default|SetMyManager Manager))

(fn ConstructionScript)

(fn IsWaveRelevant
  (return false))